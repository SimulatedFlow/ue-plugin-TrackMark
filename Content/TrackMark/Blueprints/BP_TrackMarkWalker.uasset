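; BP_TrackMarkWalker is an actor that circles its spawn point while carrying a TrackMark component, apparently as a moving source of track marks.
; BeginPlay stores the origin, passes the mark profile and surface-profile toggle to TrackMark, and applies the body material.
; Tick advances an angle by angular speed, placing the actor on the radius with yaw tangent to the circle.
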(event EventBeginPlay
  (bind _trackmark (Variables|Default|GetTrackMark))
  (Variables|Default|SetOrigin (Transformation|GetActorLocation))
  (Variables|/Script/TrackMark.TrackMarkComponent|SetProfile _trackmark (Variables|Default|GetMarkProfile))
  (Variables|/Script/TrackMark.TrackMarkComponent|SetbUseSurfaceProfiles _trackmark (Variables|Default|GetUseSurfaceProfiles))
  (Rendering|Material|SetMaterial (Variables|Default|GetBody) 0 (Variables|Default|GetBodyMaterial)))

(event Collision|EventActorBeginOverlap
  (params (OtherActor :type Actor%20Object%20Reference)))

(event EventTick
  (params (DeltaSeconds :type Float%20%28single-precision%29))
  (Variables|Default|SetAngle (+ (Variables|Default|GetAngle) (* (Variables|Default|GetAngularSpeed) DeltaSeconds)))
  (Transformation|SetActorLocationAndRotation (+ (Variables|Default|GetOrigin) (Math|Vector|RotateVector (Math|Vector|MakeVector (Variables|Default|GetRadius) 0.0 0.0) (Math|Rotator|MakeRotator 0.0 0.0 (+ (Variables|Default|GetAngle) (* (Variables|Default|GetAngularSpeed) DeltaSeconds))))) (Math|Rotator|MakeRotator 0.0 0.0 (+ (+ (Variables|Default|GetAngle) (* (Variables|Default|GetAngularSpeed) DeltaSeconds)) (Math|Float|MakeLiteralFloat 9e+01)))))

(fn ConstructionScript)