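; Demo HUD for the TrackMark system, offering buttons to change the view, scatter test marks and toggle track marks.
; On BeginPlay it sets the default track mark profile, maps snow and mud physical materials to their own profiles, and creates the buttons.
; One click handler branches on button ID to cycle the demo viewer pawn's view, spawn marks around a fixed origin, or toggle marks and update that button's label.
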(event Custom|OnButtonClicked_Event
  (params (ButtonId :type Name))
  (if (== ButtonId (Utilities|String|MakeLiteralString "view"))
    (bind _asbp_track_mark_demo_viewer (Utilities|Casting|CastToBP_TrackMarkDemoViewer (Game|Player|GetPlayerPawn 0)))
    (Default|CycleView _asbp_track_mark_demo_viewer)
    (elif (== ButtonId (Utilities|String|MakeLiteralString "scatter"))
      (Class|TrackMarkStatics|SpawnTestTrackMarks (Math|Vector|MakeVector 0.0 0.0 2.5e+02) (Variables|Default|GetScatterCount) (Variables|Default|GetScatterRadius) 0)
      (elif (== ButtonId (Utilities|String|MakeLiteralString "marks"))
        (Variables|Default|SetMarksOn (not (Variables|Default|GetMarksOn)))
        (Class|TrackMarkStatics|SetTrackMarksEnabled (not (Variables|Default|GetMarksOn)))
        (Class|TrackMarkHUD|SetButtonLabel self "marks" (select (not (Variables|Default|GetMarksOn)) (Utilities|String|MakeLiteralString "MARKS: ON") (Utilities|String|MakeLiteralString "MARKS: OFF")))))))

(event EventBeginPlay
  (bind _self self)
  (Class|TrackMarkStatics|SetDefaultTrackMarkProfile (Variables|Default|GetDefaultProfile))
  (Class|TrackMarkStatics|SetTrackMarkProfileforSurface (Variables|Default|GetSnowSurface) (Variables|Default|GetSnowProfile))
  (Class|TrackMarkStatics|SetTrackMarkProfileforSurface (Variables|Default|GetMudSurface) (Variables|Default|GetMudProfile))
  (Class|TrackMarkHUD|AddButton _self "view" "VIEW: NEXT ANGLE" "(R=0.350000,G=0.620000,B=0.950000,A=1.000000)")
  (Class|TrackMarkHUD|AddButton _self "scatter" "SCATTER MARKS" "(R=0.350000,G=0.620000,B=0.950000,A=1.000000)")
  (Class|TrackMarkHUD|AddButton _self "marks" "MARKS: ON" "(R=0.350000,G=0.620000,B=0.950000,A=1.000000)")
  (EventDispatchers|AssignOnButtonClicked _self (delegate Custom|OnButtonClicked_Event)))

(event Collision|EventActorBeginOverlap
  (params (OtherActor :type Actor%20Object%20Reference)))

(event EventTick
  (params (DeltaSeconds :type Float%20%28single-precision%29)))

(fn ConstructionScript)