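; Demo viewer actor for TrackMark that jumps between four fixed vantage points: one high view and three lower angled views.
; BeginPlay resets ViewIndex and places the actor at the high view.
; CycleView increments ViewIndex with wraparound and switches to a hard-coded location and rotation.
; The switch recomputes the increment after the store, so the shown view runs one ahead of ViewIndex.
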(event EventBeginPlay
  (Variables|Default|SetViewIndex 0)
  (Transformation|SetActorLocationAndRotation (Math|Vector|MakeVector -5.2e+03 0.0 5.6e+03) (Math|Rotator|MakeRotator 0.0 -45.0 0.0)))

(event Collision|EventActorBeginOverlap
  (params (OtherActor :type Actor%20Object%20Reference)))

(event EventTick
  (params (DeltaSeconds :type Float%20%28single-precision%29)))

(fn ConstructionScript)

(fn CycleView
  (Variables|Default|SetViewIndex (select (> (+ (Variables|Default|GetViewIndex) (Class|KismetSystemLibrary|MakeLiteralInteger 1)) (Class|KismetSystemLibrary|MakeLiteralInteger 3)) (Class|KismetSystemLibrary|MakeLiteralInteger) (+ (Variables|Default|GetViewIndex) (Class|KismetSystemLibrary|MakeLiteralInteger 1))))
  (switch int (select (> (+ (Variables|Default|GetViewIndex) (Class|KismetSystemLibrary|MakeLiteralInteger 1)) (Class|KismetSystemLibrary|MakeLiteralInteger 3)) (Class|KismetSystemLibrary|MakeLiteralInteger) (+ (Variables|Default|GetViewIndex) (Class|KismetSystemLibrary|MakeLiteralInteger 1)))
    (:0
      (Transformation|SetActorLocationAndRotation (Math|Vector|MakeVector -5.2e+03 0.0 5.6e+03) (Math|Rotator|MakeRotator 0.0 -45.0 0.0)))
    (:1
      (Transformation|SetActorLocationAndRotation (Math|Vector|MakeVector -3.6e+03 -3.6e+03 1.15e+03) (Math|Rotator|MakeRotator 0.0 -22.0 45.0)))
    (:2
      (Transformation|SetActorLocationAndRotation (Math|Vector|MakeVector -3.6e+03 0.0 1.15e+03) (Math|Rotator|MakeRotator 0.0 -22.0 45.0)))
    (:3
      (Transformation|SetActorLocationAndRotation (Math|Vector|MakeVector 0.0 0.0 1.25e+03) (Math|Rotator|MakeRotator 0.0 -22.0 45.0)))))